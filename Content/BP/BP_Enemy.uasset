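; BP_Enemy is a suicide-bomber enemy in a tank game that chases the player and self-destructs on arrival.
; After a delay, AIMoveTo targets the player controller; success triggers an explosion, camera shake, tank damage and GameMode ActorDied.
; Any incoming damage reaches the Health component, then immediately explodes and destroys the enemy without notifying GameMode.
; Tick updates the health-bar widget and turns it toward the camera.
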(event Custom|Ev_ChasePlayer
  ;[1 1 1] 플레이어와 접촉하면 2초후 자폭
  (Utilities|FlowControl|Delay 3.0)
  (AI|AIMoveTo self "0, 0, 0" (Game|GetPlayerController 0) 3e+02 true
    (:OnSuccess
      (Utilities|FlowControl|Delay 0.2)
      (Effects|SpawnEmitteratLocation "/Game/Realistic_Starter_VFX_Pack_Vol2/Particles/Explosion/P_Explosion_Big_B.P_Explosion_Big_B" (Transformation|GetActorLocation))
      (Camera|PlayWorldCameraShake "/Game/BP/BP_CameraShake.BP_CameraShake_C" (Transformation|GetActorLocation) 0.0 3e+03)
      (Actor|DestroyActor)
      (bind _asbp_pawn_tank (Utilities|Casting|CastToBP_PawnTank (Game|Player|GetPlayerPawn 0)))
      (Game|Damage|ApplyDamage _asbp_pawn_tank 5e+01 0 self "/Script/Engine.DamageType")
      (bind _asbp_tank_game_mode_base (Utilities|Casting|CastToBP_TankGameModeBase (Game|GetGameMode)))
      (Class|TankGameModeBase|ActorDied _asbp_tank_game_mode_base self))))

(event EventBeginPlay
  ;[1 1 1] 시작하자마자 플레이어를 따라와라
  (CallFunction|EvChasePlayer))

(event EventTick
  (params (DeltaSeconds :type Float%20%28single-precision%29))
  (bind _health (Variables|Default|GetHealth))
  ;[1 1 1] 몬스터 HP Widget
  (bind _aswbp_monster_hp (Utilities|Casting|CastToWBP_Monster_HP (UserInterface|GetWidget (Variables|Default|GetWidget))))
  (Default|ShowMonsterHP _aswbp_monster_hp (/ (Variables|/Script/ToonTanks.HealthComponent|GetHealth _health) (Variables|/Script/ToonTanks.HealthComponent|GetMaxHealth _health)))
  (Transformation|SetWorldRotation (Variables|Default|GetWidget) (Math|Rotator|FindLookatRotation (Transformation|GetWorldLocation (Variables|Default|GetWidget)) (Transformation|GetActorLocation (Game|GetPlayerCameraManager 0))) false false))

(event Game|Damage|EventAnyDamage
  (params (Damage :type Float%20%28single-precision%29) (DamageType :type Damage%20Type%20Object%20Reference) (InstigatedBy :type Controller%20Object%20Reference) (DamageCauser :type Actor%20Object%20Reference))
  ;[1 1 1] 적을 공격했을 때 파괴
  (Class|HealthComponent|DamageTaken (Variables|Default|GetHealth) self Damage DamageType InstigatedBy DamageCauser)
  (Effects|SpawnEmitteratLocation "/Game/Realistic_Starter_VFX_Pack_Vol2/Particles/Explosion/P_Explosion_Big_B.P_Explosion_Big_B" (Transformation|GetActorLocation))
  (Camera|PlayWorldCameraShake "/Game/BP/BP_CameraShake.BP_CameraShake_C" (Transformation|GetActorLocation) 0.0 3e+03)
  (Actor|DestroyActor))

(fn ConstructionScript)