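; BP_Spawner is an ammo spawner actor that places a BP_Ammo at its own transform on BeginPlay.
; It binds to each spawned ammo's DestroyAmmo dispatcher, though the bound function is not named.
; SpawnNewAmmo sets a five-second timer by function name to run DoSpawn, which spawns and binds another BP_Ammo.
; Only the first ammo is stored in the BPAmmo variable.
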(event EventBeginPlay
  (bind _returnvalue (Game|SpawnActorfromClass "/Game/BP/BP_Ammo.BP_Ammo_C" (Transformation|GetActorTransform self) "Undefined" "MultiplyWithRoot" 0 0))
  (Variables|Default|SetBP_Ammo _returnvalue)
  (EventDispatchers|BindEventtoEventDispatcherDestroyAmmo (Variables|Default|GetBP_Ammo) (EventDispatchers|CreateEvent :!event SpawnNewAmmo)))

(fn ConstructionScript)

(fn SpawnNewAmmo
  (Utilities|Time|SetTimerbyFunctionName 0 "DoSpawn" 5.0))

(fn DoSpawn
  (bind _returnvalue (Game|SpawnActorfromClass "/Game/BP/BP_Ammo.BP_Ammo_C" (Transformation|GetActorTransform self) "Undefined" "MultiplyWithRoot" 0 0))
  (EventDispatchers|BindEventtoEventDispatcherDestroyAmmo _returnvalue (EventDispatchers|CreateEvent :!event SpawnNewAmmo)))