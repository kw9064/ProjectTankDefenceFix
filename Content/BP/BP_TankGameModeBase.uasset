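; Tank game mode Blueprint that handles the HUD, start and end screens, and level progression.
; BeginPlay creates and stores the HP/ammo widget for the first player, while StartGame shows the start widget.
; GameOver shows the end widget with win or lose text.
; On a win, it switches on the current level name and, after a short delay, alternates between Level 1 and Level 2; a loss triggers no level change.
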(event EventBeginPlay
  (bind _returnvalue (UserInterface|CreateWidget "/Game/BP/WBP_HP_Ammo.WBP_HP_Ammo_C" (Game|GetPlayerController 0)))
  (bind _output_get (Variables|Default|SetHPWidget _returnvalue))
  (UserInterface|Viewport|AddtoViewport _output_get 0))

(event EventStartGame
  (bind _returnvalue (UserInterface|CreateWidget "/Game/BP/WBP_StartGameWidget.WBP_StartGameWidget_C"))
  (UserInterface|Viewport|AddtoViewport _returnvalue 0))

(event EventGameOver
  (params (bWonGame :type Boolean))
  (bind _output_get (Variables|Default|SetWon%20Game bWonGame))
  (bind _returnvalue (UserInterface|CreateWidget "/Game/BP/WBP_EndGameWidget.WBP_EndGameWidget_C"))
  (UserInterface|Viewport|AddtoViewport _returnvalue 0)
  (Rendering|Components|TextRender|SetText (Variables|/Game/BP/WBP_EndGameWidget.WBP_EndGameWidget_C|GetDisplayText _returnvalue) (select _output_get "YOU WIN!! 
3초뒤 이동합니다" "YOU LOSE!!"))
  (if (Variables|Default|GetWon%20Game)
    (bind _returnvalue_2 (Game|GetCurrentLevelName true))
    (switch string _returnvalue_2
      (:Level_1
        (Utilities|FlowControl|Delay 3.0)
        (Game|OpenLevel(byName) "Level_2"))
      (:Level_2
        (Utilities|FlowControl|Delay 3.0)
        (Game|OpenLevel(byName) "Level_1")))))

(fn ConstructionScript)