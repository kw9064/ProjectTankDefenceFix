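; Turret pawn Blueprint whose graph drives an overhead-style health display through its Widget component.
; Every tick it casts the widget to WBP_Monster_HP and passes it the current-to-max ratio from the Health component.
; It then rotates the widget component to face player 0's camera manager, billboarding it in world space.
; No targeting or firing logic appears here, and the construction script is empty.
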(event EventTick
  (params (DeltaSeconds :type Float%20%28single-precision%29))
  (bind _health (Variables|Default|GetHealth))
  (bind _aswbp_monster_hp (Utilities|Casting|CastToWBP_Monster_HP (UserInterface|GetWidget (Variables|Default|GetWidget))))
  (Default|ShowMonsterHP _aswbp_monster_hp (/ (Variables|/Script/ToonTanks.HealthComponent|GetHealth _health) (Variables|/Script/ToonTanks.HealthComponent|GetMaxHealth _health)))
  (Transformation|SetWorldRotation (Variables|Default|GetWidget) (Math|Rotator|FindLookatRotation (Transformation|GetWorldLocation (Variables|Default|GetWidget)) (Transformation|GetActorLocation (Game|GetPlayerCameraManager 0))) false false))

(fn ConstructionScript)