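; BP_Ammo is an ammo pickup for BP_PawnTank that bobs vertically through a Timeline played from Tick.
; The first Sphere overlap passes a DoOnce before the tank cast, so any overlapping actor uses up the single trigger.
; For a tank, it sets either MaxAmmo or CurrentAmmo depending on a SupplyAmmo threshold, then destroys itself and calls the DestroyAmmo dispatcher.
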(event OnComponentBeginOverlap(Sphere)
  (params (OverlappedComponent :type Primitive%20Component%20Object%20Reference) (OtherActor :type Actor%20Object%20Reference) (OtherComp :type Primitive%20Component%20Object%20Reference) (OtherBodyIndex :type Integer) (bFromSweep :type Boolean) (SweepResult :type Hit%20Result%20Structure%20%28by%20ref%29))
  (Utilities|FlowControl|DoOnce false
    (:Completed
      (bind _asbp_pawn_tank (Utilities|Casting|CastToBP_PawnTank OtherActor))
      (if (> (+ 0 (Variables|Default|GetSupplyAmmo)) 20)
        (Variables|/Script/ToonTanks.Tank|SetMaxAmmo _asbp_pawn_tank (Variables|Default|GetMax%20Ammo))
        (else
          (Variables|/Script/ToonTanks.Tank|SetCurrentAmmo _asbp_pawn_tank (Variables|Default|GetCurrent%20Ammo))))
      (Actor|DestroyActor)
      (Default|CallEventDispatcherDestroyAmmo))))

(event EventTick
  (params (DeltaSeconds :type Float%20%28single-precision%29))
  ;[1 1 1] Ammo 애니메이션
  (bind _newtrack_0 (Timeline|Timeline Play)
    (:Update
      (Transformation|SetRelativeLocation (Variables|Default|GetStaticMesh) (Math|Vector|MakeVector 0.0 0.0 (* _newtrack_0 5e+01)) false false))))

(fn ConstructionScript)